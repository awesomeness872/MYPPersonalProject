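; Base Blueprint for gun pickups that equip a weapon on the player's character when used.
; The construction script applies the gun's static mesh and fills in the pickup's image, name, description and action text from variables.
; On UseItem, it casts player 0's character to BP_MainCharacter and calls SwitchGun, passing the gun type, firing stats, skeletal mesh and attachment transform.
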(event `self.ReceiveBeginPlay`)

(event `self.UseItem`
  (bind _asbp_main_character (cast `/Game/Blueprints/BP_MainCharacter` (`GameplayStatics.GetPlayerCharacter` 0)))
  (`MainCharacter.SwitchGun` _asbp_main_character (`self.GunType`) (`self.MaxAmmo`) (`self.DamagePerRound`) (`self.RateOfFire`) (`self.IsAutomatic`) (`self.GunSkMesh`) (`self.GunOffset`) (`self.GunRotation`) (`self.GunScale`)))

(fn `UserConstructionScript`
  (`StaticMeshComponent.SetStaticMesh` (`self.PickupMesh`) (`self.GunMesh`))
  (`self.SetPickupImage` (`self.GunImage`))
  (`self.SetPickupName` (`self.GunName`))
  (`self.SetPickupDescription` (`self.GunDescription`))
  (`self.SetActionText` (`self.GunActionText`)))