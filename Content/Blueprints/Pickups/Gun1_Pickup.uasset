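; Gun pickup that equips the player with a specific weapon when its UseItem event fires.
; It casts the player character to BP_MainCharacter and copies over its ammo capacity, damage, fire rate, automatic flag and gun mesh.
; It then applies a hard-coded rotation and scale to the character's gun component to fit the mesh.
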(event `self.ReceiveBeginPlay`)

(event `self.UseItem`
  (bind _asbp_main_character (cast `/Game/Blueprints/BP_MainCharacter` (`GameplayStatics.GetPlayerCharacter` 0)))
  (`MainCharacter.SetMaxAmmo` _asbp_main_character (`self.MaxAmmo`))
  (`MainCharacter.SetDamagePerRound` _asbp_main_character (`self.DamagePerRound`))
  (`MainCharacter.SetRateOfFire` _asbp_main_character (`self.RateOfFire`))
  (`MainCharacter.SetIsAutomaticWeapon` _asbp_main_character (`self.bIsAutomatic`))
  (`MainCharacter.SetGunMesh` _asbp_main_character (`self.GunMesh`))
  (bind _returnvalue (`MainCharacter.GetGunComp` _asbp_main_character))
  (`SceneComponent.K2_SetRelativeLocationAndRotation` _returnvalue (0.0 0.0 0.0) (struct :`Yaw` -60.0) false false)
  (`SceneComponent.SetRelativeScale3D` _returnvalue (2.0 2.0 2.0)))

(fn `UserConstructionScript`)