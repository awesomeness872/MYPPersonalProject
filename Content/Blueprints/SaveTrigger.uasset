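; SaveTrigger is a trigger volume that saves the game through BP_MainCharacter when the player is inside and no living enemies are counted.
; On player overlap it counts non-dead enemies in EnemyCheckBox into AliveCount, saving immediately if none are found or the count is zero.
; Tick also saves through a DoOnce while PlayerInside and AliveCount is zero, resetting it otherwise.
; This graph only increments AliveCount, never decrementing or resetting it.
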(event `self.ReceiveTick`
  (params (DeltaSeconds :type "Float (single-precision)"))
  ;[1 1 1] If player is inside and enemies are killed, save the game
  (if (and (`self.PlayerInside`) (== (`self.AliveCount`) 0))
    (`/Engine/EditorBlueprintResources/StandardMacros.DoOnce` false :!label _label
      (:`Completed`
        (bind _asbp_main_character (cast `/Game/Blueprints/BP_MainCharacter` (`GameplayStatics.GetPlayerPawn` 0)))
        (`MainCharacter.SaveGame` _asbp_main_character)))
    (else
      (goto _label :!via `Reset`))))

(event `self.CollisionComponent.OnComponentBeginOverlap`
  (params (OverlappedComponent :type "PrimitiveComponent Object Reference") (OtherActor :type "Actor Object Reference") (OtherComp :type "PrimitiveComponent Object Reference") (OtherBodyIndex :type Integer) (bFromSweep :type Boolean) (SweepResult :type "HitResult Structure (by ref)"))
  (bind _returnvalue (`GameplayStatics.GetPlayerPawn` 0))
  (bind _overlappingactors (`PrimitiveComponent.GetOverlappingActors` (`self.EnemyCheckBox`) "/Script/RPGProject.EnemyCharacter"))
  ;[1 1 1] When player steps in to area, save game
  (if (== OtherActor _returnvalue)
    (set `self.PlayerInside` true)
    (if (== (`KismetArrayLibrary.Array_Length` _overlappingactors) 0)
      (bind _asbp_main_character (cast `/Game/Blueprints/BP_MainCharacter` _returnvalue))
      (`MainCharacter.SaveGame` _asbp_main_character)
      (else
        ;;[1 1 1] If no enemies are alive, save game
        (for _array_element _overlappingactors
          (bind _asbp_enemy_character (cast `/Game/Blueprints/Enemies/BP_EnemyCharacter` _array_element))
          (bind _returnvalue_2 (`EnemyCharacter.GetDead` _asbp_enemy_character))
          (if (not _returnvalue_2)
            (`/Engine/EditorBlueprintResources/StandardMacros.IncrementInt` (`self.AliveCount`))))
        (if (== (`self.AliveCount`) 0)
          (bind _asbp_main_character_2 (cast `/Game/Blueprints/BP_MainCharacter` (`GameplayStatics.GetPlayerPawn` 0)))
          (`MainCharacter.SaveGame` _asbp_main_character_2))))))

(event `self.CollisionComponent.OnComponentEndOverlap`
  (params (OverlappedComponent :type "PrimitiveComponent Object Reference") (OtherActor :type "Actor Object Reference") (OtherComp :type "PrimitiveComponent Object Reference") (OtherBodyIndex :type Integer))
  ;[1 1 1] Set PlayerInside to false when player leaves
  (if (== OtherActor (`GameplayStatics.GetPlayerPawn` 0))
    (set `self.PlayerInside` false)))

(fn `UserConstructionScript`)