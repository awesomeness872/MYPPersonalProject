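; DoubleDoorManual is an interactive double sliding door that opens and closes each time it is activated.
; The Activate event runs a FlipFlop that alternates between open and closed.
; Each state slides LeftDoor and RightDoor to fixed relative positions with eased MoveComponentTo calls over half a second.
; It also sets ActionText to name the next available action.
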(event `self.Activate`
  (`/Engine/EditorBlueprintResources/StandardMacros.FlipFlop`
    (:`A`
      ;[1 1 1] Move doors to open position and set action to close doors
      (`|ExecutionSequence`
        (:`then_0`
          (`KismetSystemLibrary.MoveComponentTo` (`self.LeftDoor`) (0.0 -228.0 150.0) (struct) true true 0.5))
        (:`then_1`
          (`KismetSystemLibrary.MoveComponentTo` (`self.RightDoor`) (0.0 201.0 150.0) (struct) true true 0.5))
        (:`then_2`
          (set `self.ActionText` "Close Doors"))))
    (:`B`
      ;[1 1 1] Move doors to closed position and set action to open doors
      (`|ExecutionSequence`
        (:`then_0`
          (`KismetSystemLibrary.MoveComponentTo` (`self.LeftDoor`) (0.0 -89.0 150.0) (struct) true true 0.5))
        (:`then_1`
          (`KismetSystemLibrary.MoveComponentTo` (`self.RightDoor`) (0.0 61.0 150.0) (struct) true true 0.5))
        (:`then_2`
          (set `self.ActionText` "Open Doors"))))))

(fn `UserConstructionScript`)